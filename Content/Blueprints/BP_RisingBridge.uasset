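; Bridge actor that rises once when its linked switch is activated.
; BeginPlay binds to LinkSwitch, lowers the mesh, then caches a base height offset further below that lowered position.
; Activation plays a timeline that lerps the mesh's Z up from the cached base using teleport moves.
; Rising and risen flags block retriggering, so the bridge never lowers again.
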(event `self.ReceiveBeginPlay`
  (bind _mesh_0 (`self.Mesh_0`))
  (bind (_returnvalue_x _returnvalue_y _returnvalue_z) (`KismetMathLibrary.BreakVector` (`SceneComponent.K2_GetComponentLocation` _mesh_0)))
  (bind _returnvalue (- _returnvalue_z 125.0))
  (add `/Game/Blueprints/BP_RisingBridgeSwitch.switchActivated` (`self.linkSwitch`) (delegate `switchActivated`))
  (`SceneComponent.K2_SetWorldLocation` _mesh_0 (`KismetMathLibrary.MakeVector` _returnvalue_x _returnvalue_y _returnvalue) false true)
  (set `self.bridgeZ` _returnvalue))

(event `switchActivated`
  (bind _bridgez (`self.bridgeZ`))
  (bind _mesh_0 (`self.Mesh_0`))
  (bind (_returnvalue_x _returnvalue_y) (`KismetMathLibrary.BreakVector` (`SceneComponent.K2_GetComponentLocation` _mesh_0)))
  (if (not (or (`self.bridgeRising`) (`self.isRisen`)))
    (set `self.bridgeRising` true)
    (bind (_direction _bridge_ztrack) (`Timeline|Timeline_BridgeRising` :!via `PlayFromStart`)
      (:`Update`
        (`SceneComponent.K2_SetWorldLocation` _mesh_0 (`KismetMathLibrary.MakeVector` _returnvalue_x _returnvalue_y (`KismetMathLibrary.Lerp` _bridgez (+ _bridgez 250.0) _bridge_ztrack)) false true))
      (:`Finished`
        (set `self.bridgeRising` false)
        (set `self.isRisen` true)))))

(fn `UserConstructionScript`)