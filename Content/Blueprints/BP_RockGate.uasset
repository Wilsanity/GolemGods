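; BP_RockGate is a rock gate actor that opens by sinking its static mesh downward.
; OpenGate, when the gate is closed, plays a timeline that lerps the mesh's relative Z from raised to lowered, teleporting it each update, then clears IsClosed.
; The construction script uses IsClosed to place the mesh raised or lowered, so the initial state shows on placed instances.
; No closing logic is present.
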(event `OpenGate`
  (bind _staticmesh (`self.StaticMesh`))
  (bind (_relativelocation_x _relativelocation_y) (`KismetMathLibrary.BreakVector` (`SceneComponent.RelativeLocation` _staticmesh)))
  (if (`self.isClosed`)
    (set `self.opening` true)
    (bind (_direction _time) (`Timeline|TL_LowerGate` :!via `PlayFromStart`)
      (:`Update`
        (`SceneComponent.K2_SetRelativeLocation` _staticmesh (`KismetMathLibrary.MakeVector` _relativelocation_x _relativelocation_y (`KismetMathLibrary.Lerp` 0.0 -640.0 _time)) false true))
      (:`Finished`
        (set `self.opening` false)
        (set `self.isClosed` false)))))

(fn `UserConstructionScript`
  (bind _staticmesh (`self.StaticMesh`))
  (if (`self.isClosed`)
    (`SceneComponent.K2_SetRelativeLocation` _staticmesh (0.0 0.0 0.0) false true)
    (else
      (`SceneComponent.K2_SetRelativeLocation` _staticmesh (0.0 0.0 -640.0) false true))))