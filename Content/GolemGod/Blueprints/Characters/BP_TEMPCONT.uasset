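; Temporary player controller that drives a BP_TEMPPAWN with legacy axis inputs for movement and camera look.
; Move axes offset the pawn along its camera's forward and right vectors, scaled by MoveSpeed and delta time, with sweep.
; The camera axis adds scaled pitch and yaw to the spring arm's world rotation, zeroing roll, without clamping.
; Interact and MoveDown inputs only print debug strings.
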(event `self.ReceiveBeginPlay`)

(event `EnhancedInput|/Game/GolemGod/Blueprints/Input/input_Interact`
  (params (ActionValue :type Boolean) (ElapsedSeconds :type "Float (double-precision)") (TriggeredSeconds :type "Float (double-precision)") (InputAction :type "InputAction Object Reference" :default "/Game/GolemGod/Blueprints/Input/input_Interact.input_Interact"))
  (:`Triggered`
    (`KismetSystemLibrary.PrintString` "Hello")))

(event `EnhancedInput|/Game/GolemGod/Blueprints/Input/input_MoveDown`
  (params (ActionValue :type "Vector2D Structure") (ElapsedSeconds :type "Float (double-precision)") (TriggeredSeconds :type "Float (double-precision)") (InputAction :type "InputAction Object Reference" :default "/Game/GolemGod/Blueprints/Input/input_MoveDown.input_MoveDown"))
  (:`Triggered`
    (`KismetSystemLibrary.PrintString` "Up")
    (cast `/Game/GolemGod/Blueprints/Characters/BP_TEMPPAWN` (`self.K2_GetPawn`))))

(event `InputAxis|legacy_moveY`
  (params (AxisValue :type "Float (single-precision)"))
  (bind _asbp_temppawn (cast `/Game/GolemGod/Blueprints/Characters/BP_TEMPPAWN` (`self.K2_GetPawn`)))
  (`self.K2_AddActorWorldOffset` _asbp_temppawn (* (`SceneComponent.GetForwardVector` (`/Game/GolemGod/Blueprints/Characters/BP_TEMPPAWN.Camera` _asbp_temppawn)) AxisValue (`/Game/GolemGod/Blueprints/Characters/BP_TEMPPAWN.moveSpeed` _asbp_temppawn) (`GameplayStatics.GetWorldDeltaSeconds`)) true true))

(event `InputAxis|legacy_moveX`
  (params (AxisValue :type "Float (single-precision)"))
  (bind _asbp_temppawn (cast `/Game/GolemGod/Blueprints/Characters/BP_TEMPPAWN` (`self.K2_GetPawn`)))
  (`self.K2_AddActorWorldOffset` _asbp_temppawn (* (`SceneComponent.GetRightVector` (`/Game/GolemGod/Blueprints/Characters/BP_TEMPPAWN.Camera` _asbp_temppawn)) AxisValue (`/Game/GolemGod/Blueprints/Characters/BP_TEMPPAWN.moveSpeed` _asbp_temppawn) (`GameplayStatics.GetWorldDeltaSeconds`)) true true))

(event `InputAxis|legacy_moveCameraXY`
  (params (AxisValue :type "Float (single-precision)"))
  (bind _asbp_temppawn (cast `/Game/GolemGod/Blueprints/Characters/BP_TEMPPAWN` (`self.K2_GetPawn`)))
  (bind _springarm (`/Game/GolemGod/Blueprints/Characters/BP_TEMPPAWN.SpringArm` _asbp_temppawn))
  (`SceneComponent.K2_SetWorldRotation` _springarm (`KismetMathLibrary.MakeRotator` 0.0 (+ (.pitch (`SceneComponent.K2_GetComponentRotation` _springarm)) (* (`self.GetInputAxisValue`) 15.0)) (+ (.yaw (`SceneComponent.K2_GetComponentRotation` _springarm)) (* (`self.GetInputAxisValue`) 15.0))) false false))

(fn `UserConstructionScript`)